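; BP_PlayableGameCharacter is the playable character Blueprint, handling damage pop-ups, the health bar and initial spell selection.
; After a short BeginPlay delay it binds the damage delegate, then writes the first Spells entry into each looped SelectedSpells index, printing its validity.
; Damage events create a WBP_DamagePop showing amount, critical and miss state in the DamagePop widget component.
; Tick polls HealthComponent to update the WBP_HealthBar percentage.
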(event Custom|DisplayDamage
  (params (Damage :type Integer) (Critic :type Boolean) (Missed :type Boolean))
  (bind _returnvalue (UserInterface|CreateWidget "/Game/UI/DungeonUI/ActorsUI/WBP_DamagePop.WBP_DamagePop_C" 0 Damage Critic Missed))
  (UserInterface|SetWidget (Variables|Default|GetDamagePop) _returnvalue))

(event EventBeginPlay
  (bind _spells (Variables|Default|GetSpells))
  (bind _output (Utilities|Array|Get(acopy) _spells))
  (|CallParentFunction)
  (Utilities|FlowControl|Delay 0.1)
  (EventDispatchers|BindEventtoOnDamageTakenDelegate (delegate Custom|DisplayDamage))
  (for _index (range 0 (Utilities|Array|Length _spells))
    (Utilities|Array|SetArrayElem (Variables|Default|GetSelectedSpells) _index _output)
    (Development|PrintString (Utilities|String|ToString(Boolean) (Utilities|IsValid _output)))))

(event EventTick
  (params (DeltaSeconds :type Float%20%28single-precision%29))
  (bind _healthcomponent (Variables|Default|GetHealthComponent))
  (bind _aswbp_health_bar (Utilities|Casting|CastToWBP_HealthBar (UserInterface|GetWidget (Variables|Default|GetHealthBar))))
  (Default|SetHealthPercent _aswbp_health_bar (/ (Math|Conversions|ToFloat(Integer) (Variables|/Script/Dungeon_Crawler.HealthComponent|GetCurrentHealth _healthcomponent)) (Math|Conversions|ToFloat(Integer) (Variables|/Script/Dungeon_Crawler.HealthComponent|GetMaxHealth _healthcomponent)))))

(fn ConstructionScript)