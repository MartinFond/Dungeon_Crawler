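; BP_EnemyGameCharacter is an enemy character that shows its health and the damage it takes through widget components.
; On BeginPlay it binds to a damage-taken delegate, creating a new WBP_DamagePop for each hit with amount, critical and missed flags and assigning it to the DamagePop component.
; Every Tick it polls HealthComponent and pushes the current-to-max health ratio into the WBP_HealthBar widget.
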(event Custom|DisplayDamage
  (params (Damage :type Integer) (Critic :type Boolean) (Missed :type Boolean))
  (bind _returnvalue (UserInterface|CreateWidget "/Game/UI/DungeonUI/ActorsUI/WBP_DamagePop.WBP_DamagePop_C" 0 Damage Critic Missed))
  (UserInterface|SetWidget (Variables|Default|GetDamagePop) _returnvalue))

(event EventBeginPlay
  (EventDispatchers|BindEventtoOnDamageTakenDelegate (delegate Custom|DisplayDamage)))

(event EventTick
  (params (DeltaSeconds :type Float%20%28single-precision%29))
  (bind _healthcomponent (Variables|Default|GetHealthComponent))
  (bind _aswbp_health_bar (Utilities|Casting|CastToWBP_HealthBar (UserInterface|GetWidget (Variables|Default|GetHealthBar))))
  (Default|SetHealthPercent _aswbp_health_bar (/ (Math|Conversions|ToFloat(Integer) (Variables|/Script/Dungeon_Crawler.HealthComponent|GetCurrentHealth _healthcomponent)) (Math|Conversions|ToFloat(Integer) (Variables|/Script/Dungeon_Crawler.HealthComponent|GetMaxHealth _healthcomponent)))))

(fn ConstructionScript)