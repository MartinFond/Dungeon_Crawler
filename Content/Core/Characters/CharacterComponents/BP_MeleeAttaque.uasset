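; BP_MeleeAttaque is a character component that casts a melee attack on the character occupying the player controller's hovered cell.
; CastSpell runs range and hit checks, then generates damage and doubles it on a critical.
; Hits apply physical damage through ApplyDamage.
; Hits and misses are reported through the enemy character's damage-taken delegate, while an out-of-range target gets no response beyond a leftover debug print.
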(event EventBeginPlay
  (|CallParentFunction) ; This node is disabled and will not be called.\nDrag off pins to build functionality.
)

(event EventTick
  (params (DeltaSeconds :type Float%20%28single-precision%29))
  (|CallParentFunction DeltaSeconds) ; This node is disabled and will not be called.\nDrag off pins to build functionality.
)

(event EventCastSpell
  (Development|PrintString "Hello")
  (bind _asbp_dungeon_player_controller (Utilities|Casting|CastToBP_DungeonPlayerController (Game|GetPlayerController 0)))
  (Utilities|IsValid (Variables|/Script/Dungeon_Crawler.HexCell|GetOccupierCharacter (Variables|/Script/Dungeon_Crawler.DungeonPlayerController|GetOveredCell _asbp_dungeon_player_controller))
    (:Is%20Valid
      (bind _returnvalue (Class|BaseSpellComponent|CheckRange (Variables|/Script/Dungeon_Crawler.HexCell|GetOccupierCharacter (Variables|/Script/Dungeon_Crawler.DungeonPlayerController|GetOveredCell _asbp_dungeon_player_controller))))
      (if _returnvalue
        (bind _returnvalue_2 (Class|BaseSpellComponent|CheckHit (Variables|/Script/Dungeon_Crawler.HexCell|GetOccupierCharacter (Variables|/Script/Dungeon_Crawler.DungeonPlayerController|GetOveredCell _asbp_dungeon_player_controller))))
        (if _returnvalue_2
          (bind _returnvalue_3 (Class|BaseSpellComponent|GenerateDamage))
          (bind _returnvalue_4 (Class|BaseSpellComponent|CheckCritic))
          (if _returnvalue_4
            (bind _output_get (Variables|Default|SetDamage (* _returnvalue_3 2)))
            (else
              (Variables|Default|SetDamage _returnvalue_3)))
          (bind _returnvalue_5 (Game|Damage|ApplyDamage (Variables|/Script/Dungeon_Crawler.HexCell|GetOccupierCharacter (Variables|/Script/Dungeon_Crawler.DungeonPlayerController|GetOveredCell _asbp_dungeon_player_controller)) (Math|Conversions|ToFloat(Integer) _output_get) 0 (Components|GetOwner) "/Script/Dungeon_Crawler.PhysicalDamage"))
          (bind _asbp_enemy_game_character (Utilities|Casting|CastToBP_EnemyGameCharacter (Variables|/Script/Dungeon_Crawler.HexCell|GetOccupierCharacter (Variables|/Script/Dungeon_Crawler.DungeonPlayerController|GetOveredCell _asbp_dungeon_player_controller))))
          (Default|CallOnDamageTakenDelegate _asbp_enemy_game_character (Math|Float|Truncate _returnvalue_5) _returnvalue_4 false)
          (else
            (bind _asbp_enemy_game_character_2 (Utilities|Casting|CastToBP_EnemyGameCharacter (Variables|/Script/Dungeon_Crawler.HexCell|GetOccupierCharacter (Variables|/Script/Dungeon_Crawler.DungeonPlayerController|GetOveredCell _asbp_dungeon_player_controller))))
            (Default|CallOnDamageTakenDelegate _asbp_enemy_game_character_2 0 false true)))))))