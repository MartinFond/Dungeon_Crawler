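; Warrior Charge spell that rushes the caster along a straight hex line toward the character on the hovered cell.
; CastSpell sums walking costs of the cells between both characters and, if within the caster's Speed, sends that path minus the target's cell to the AI controller.
; Without waiting for movement, it rolls a hit, scaling DamageRatio by cells crossed for physical damage, and displays damage or a miss on enemy targets.
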(event EventBeginPlay)

(event EventTick
  (params (DeltaSeconds :type Float%20%28single-precision%29)))

(event EventCastSpell
  (bind _asbp_dungeon_player_controller (Utilities|Casting|CastToBP_DungeonPlayerController (Game|GetPlayerController 0)))
  (Utilities|IsValid (Variables|/Script/Dungeon_Crawler.HexCell|GetOccupierCharacter (Variables|/Script/Dungeon_Crawler.DungeonPlayerController|GetOveredCell _asbp_dungeon_player_controller))
    (:Is%20Valid
      (Variables|Default|SetSpellTarget (Variables|/Script/Dungeon_Crawler.HexCell|GetOccupierCharacter (Variables|/Script/Dungeon_Crawler.DungeonPlayerController|GetOveredCell _asbp_dungeon_player_controller)))
      (Variables|Default|SetRangeMax (+ (Variables|/Script/Dungeon_Crawler.CharacterInfo|GetSpeed (Variables|/Script/Dungeon_Crawler.GameCharacter|GetCharacterInfo (Variables|Default|GetSpellCaster))) 1))
      (Class|BaseSpellComponent|CheckRange (Variables|Default|GetSpellTarget))
      (bind _output_get (Variables|Default|SetPath (Class|HexGrid|LinePath (Variables|/Script/Dungeon_Crawler.DungeonPlayerController|GetHexGrid _asbp_dungeon_player_controller) (Variables|/Script/Dungeon_Crawler.GameCharacter|GetHexLocation (Variables|Default|GetSpellCaster)) (Variables|/Script/Dungeon_Crawler.GameCharacter|GetHexLocation (Variables|Default|GetSpellTarget)))))
      (for (_array_element _array_index) (Class|HexGrid|LinePath (Variables|/Script/Dungeon_Crawler.DungeonPlayerController|GetHexGrid _asbp_dungeon_player_controller) (Variables|/Script/Dungeon_Crawler.GameCharacter|GetHexLocation (Variables|Default|GetSpellCaster)) (Variables|/Script/Dungeon_Crawler.GameCharacter|GetHexLocation (Variables|Default|GetSpellTarget)))
        (if (and (!= _array_index 0) (!= (- (Utilities|Array|Length (Class|HexGrid|LinePath (Variables|/Script/Dungeon_Crawler.DungeonPlayerController|GetHexGrid _asbp_dungeon_player_controller) (Variables|/Script/Dungeon_Crawler.GameCharacter|GetHexLocation (Variables|Default|GetSpellCaster)) (Variables|/Script/Dungeon_Crawler.GameCharacter|GetHexLocation (Variables|Default|GetSpellTarget)))) 1) _array_index))
          (Variables|Default|SetPathLength (+ (Class|HexCell|GetMovementCost _array_element "Walking") (Variables|Default|GetPathLength)))))
      (if (<= (Variables|Default|GetPathLength) (Variables|/Script/Dungeon_Crawler.CharacterInfo|GetSpeed (Variables|/Script/Dungeon_Crawler.GameCharacter|GetCharacterInfo (Variables|Default|GetSpellCaster))))
        (bind _ascharacter_aicontroller (Utilities|Casting|CastToCharacterAIController (Pawn|GetController (Variables|Default|GetSpellCaster))))
        (Utilities|Array|RemoveIndex _output_get (- (Utilities|Array|Length (Class|HexGrid|LinePath (Variables|/Script/Dungeon_Crawler.DungeonPlayerController|GetHexGrid _asbp_dungeon_player_controller) (Variables|/Script/Dungeon_Crawler.GameCharacter|GetHexLocation (Variables|Default|GetSpellCaster)) (Variables|/Script/Dungeon_Crawler.GameCharacter|GetHexLocation (Variables|Default|GetSpellTarget)))) 1))
        (Class|CharacterAIController|CustomPathMove _ascharacter_aicontroller (Variables|Default|GetPath))
        (bind _returnvalue (Class|BaseSpellComponent|CheckHit (Variables|Default|GetSpellTarget)))
        (bind _asbp_enemy_game_character (Utilities|Casting|CastToBP_EnemyGameCharacter (Variables|Default|GetSpellTarget)))
        (if _returnvalue
          (Variables|Default|SetDamageRatio (* (- (Utilities|Array|Length (Class|HexGrid|LinePath (Variables|/Script/Dungeon_Crawler.DungeonPlayerController|GetHexGrid _asbp_dungeon_player_controller) (Variables|/Script/Dungeon_Crawler.GameCharacter|GetHexLocation (Variables|Default|GetSpellCaster)) (Variables|/Script/Dungeon_Crawler.GameCharacter|GetHexLocation (Variables|Default|GetSpellTarget)))) 2) 5))
          (bind _returnvalue_2 (Class|BaseSpellComponent|GenerateDamage))
          (Game|Damage|ApplyDamage 0 (Math|Conversions|ToFloat(Integer) _returnvalue_2) 0 (Components|GetOwner) "/Script/Dungeon_Crawler.PhysicalDamage")
          (Default|DisplayDamage _asbp_enemy_game_character (Math|Float|Truncate (Math|Conversions|ToFloat(Integer) _returnvalue_2)) false false false)
          (else
            (Default|DisplayDamage _asbp_enemy_game_character 0 false true false)))))))