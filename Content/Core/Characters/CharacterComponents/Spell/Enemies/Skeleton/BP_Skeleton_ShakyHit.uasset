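; Skeleton enemy spell "Shaky Hit", a single-target physical attack run when the spell is cast.
; CastSpell checks range, then rolls for hit, generates damage and doubles it on a critical.
; A hit applies physical damage to SpellTarget and reports the applied amount and critical flag through its damage-taken delegate.
; A miss reports zero damage as missed, while an out-of-range cast does nothing.
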(event EventBeginPlay)

(event EventTick
  (params (DeltaSeconds :type Float%20%28single-precision%29)))

(event EventCastSpell
  (bind _spelltarget (Variables|Default|GetSpellTarget))
  (if true
    (bind _returnvalue (Class|SingleTargetSpellComponent|CheckRangeSingle))
    (if _returnvalue
      (bind _returnvalue_2 (Class|SingleTargetSpellComponent|CheckHitSingle))
      (if _returnvalue_2
        (bind _returnvalue_3 (Class|BaseSpellComponent|GenerateDamage))
        (bind _returnvalue_4 (Class|BaseSpellComponent|CheckCritic))
        (if _returnvalue_4
          (bind _output_get (Variables|Default|SetDamage (* _returnvalue_3 2)))
          (else
            (Variables|Default|SetDamage _returnvalue_3)))
        (bind _returnvalue_5 (Game|Damage|ApplyDamage _spelltarget (Math|Conversions|ToFloat(Integer) _output_get) 0 0 "/Script/Dungeon_Crawler.PhysicalDamage"))
        (Default|CallOnDamageTakenDelegate _spelltarget (Math|Float|Truncate _returnvalue_5) _returnvalue_4 false)
        (else
          (Default|CallOnDamageTakenDelegate (Variables|Default|GetSpellTarget) 0 false true))))))