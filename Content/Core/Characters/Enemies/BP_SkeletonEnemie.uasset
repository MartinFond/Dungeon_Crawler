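; Skeleton enemy for a turn-based hex-grid dungeon game that approaches an ally and casts Shaky Hit on it.
; It binds to the game mode's begin-turn delegate and, when active, runs a delayed move, cast, end-turn, begin-next-turn sequence.
; Targeting filters Allies by A* path length, then health, but never updates either running best value.
; Non-adjacent targets are approached through the AI controller's limited-range A* move.
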(event Custom|Move
  (bind _closestenemies (Variables|Default|GetClosestEnemies))
  (bind _closestenemies_2 (Variables|Default|GetClosestEnemies))
  (bind _asdungeon_game_mode (Utilities|Casting|CastToDungeonGameMode (Game|GetGameMode)))
  (Variables|Default|SetClosestEnnemiesDistance 100)
  (for _array_element (Variables|/Script/Dungeon_Crawler.DungeonGameMode|GetAllies _asdungeon_game_mode)
    (if (== (Utilities|Array|Length (Class|HexGrid|AStarPath (Variables|Default|GetHexGrid) (Variables|Default|GetHexLocation) (Variables|/Script/Dungeon_Crawler.GameCharacter|GetHexLocation _array_element) "Walking")) (Variables|Default|GetClosestEnnemiesDistance))
      (Utilities|Array|Add _closestenemies _array_element)
      (elif (< (Utilities|Array|Length (Class|HexGrid|AStarPath (Variables|Default|GetHexGrid) (Variables|Default|GetHexLocation) (Variables|/Script/Dungeon_Crawler.GameCharacter|GetHexLocation _array_element) "Walking")) (Variables|Default|GetClosestEnnemiesDistance))
        (Utilities|Array|Clear _closestenemies)
        (Utilities|Array|Add _closestenemies _array_element))))
  (Development|PrintString (Utilities|String|ToString(Integer) (Utilities|Array|Length _closestenemies_2)))
  (bind _output_get (Variables|Default|SetTargetEnemyHealth 0))
  (for _array_element_2 _closestenemies_2
    (if (> (Variables|/Script/Dungeon_Crawler.HealthComponent|GetCurrentHealth (Variables|/Script/Dungeon_Crawler.GameCharacter|GetHealthComponent _array_element_2)) _output_get)
      (Variables|Default|SetTargetEnemy _array_element_2)
      (Development|PrintString "Target Set")))
  (if (not (<= (Class|HexCell|Distance (Variables|Default|GetHexLocation) (Variables|/Script/Dungeon_Crawler.GameCharacter|GetHexLocation (Variables|Default|GetTargetEnemy))) 1.0))
    (bind _ascharacter_aicontroller (Utilities|Casting|CastToCharacterAIController (AI|GetAIController self))
      (:then
        (Class|CharacterAIController|AStarMove _ascharacter_aicontroller (Variables|/Script/Dungeon_Crawler.GameCharacter|GetHexLocation (Variables|Default|GetTargetEnemy)) 3)
        (Development|PrintString "Moved !"))
      (:CastFailed
        (Development|PrintString "CastFailed")))))

(event Custom|CastShakyHit
  (bind _bp_skeleton_shakyhit (Variables|Default|GetBP_Skeleton_ShakyHit))
  (Variables|/Script/Dungeon_Crawler.SingleTargetSpellComponent|SetSpellTarget _bp_skeleton_shakyhit (Variables|Default|GetTargetEnemy))
  (Class|BaseSpellComponent|CastSpell _bp_skeleton_shakyhit))

(event Custom|MoveAndAttaque
  (if (== (Variables|/Script/Dungeon_Crawler.DungeonGameMode|GetCurrentActiveCharacter (stale EventBeginPlay _asdungeon_game_mode)) self)
    (Utilities|FlowControl|Delay 0.2)
    (CallFunction|Move)
    (Utilities|FlowControl|Delay 0.5)
    (CallFunction|CastShakyHit)
    (Utilities|FlowControl|Delay 0.2)
    (bind _asdungeon_game_mode (Utilities|Casting|CastToDungeonGameMode (Game|GetGameMode)))
    (Utilities|FlowControl|Delay 0.1)
    (Class|DungeonGameMode|EndTurn _asdungeon_game_mode)
    (Utilities|FlowControl|Delay 0.1)
    (Class|DungeonGameMode|BeginTurn _asdungeon_game_mode)))

(event EventBeginPlay
  (|CallParentFunction)
  (bind _asdungeon_game_mode (Utilities|Casting|CastToDungeonGameMode (Game|GetGameMode)))
  (EventDispatchers|BindEventtoBeginTurnDelegate _asdungeon_game_mode (delegate Custom|MoveAndAttaque)))

(event Collision|EventActorBeginOverlap
  (params (OtherActor :type Actor%20Object%20Reference)))

(event EventTick
  (params (DeltaSeconds :type Float%20%28single-precision%29))
  (|CallParentFunction DeltaSeconds) ; This node is disabled and will not be called.\nDrag off pins to build functionality.
)

(fn ConstructionScript
  (|CallParentFunction))